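; Physics-driven rowable boat that can be upgraded with extra seats.
; Row events apply force and yaw torque to the Sphere by paddle direction, while Tick zeroes its roll and pitch.
; Upgrading, via a server-gated event or a multicast one, shifts Front and Tail and attaches a new BP_Seat to Front.
; Tick also calls velocity-to-heading alignment, but that logic is disconnected and never runs.
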(event Custom|MULTICAST_UpgradeBoat
  (Transformation|AddRelativeLocation (Variables|Default|GetFront) "10.000000,10.000000,0.000000" false false)
  (Transformation|AddRelativeLocation (Variables|Default|GetTail) "0.000000,-20.000000, 0" false false)
  (bind _returnvalue (AddComponent|AddChildActorComponent false))
  (ChildActorComponent|SetChildActorClass _returnvalue "/Game/ThirdPersonCPP/Blueprints/BoatActorMethod/BP_Seat.BP_Seat_C")
  (Transformation|AttachComponentToComponent _returnvalue (Variables|Default|GetFront) "None" "KeepWorld" "KeepWorld" "KeepWorld" true)
  (Transformation|SetRelativeLocation _returnvalue (Variables|/Script/Engine.SceneComponent|GetRelativeLocation (Variables|Default|GetTail)) false false))

(event Custom|Row!
  (params (PropulsionDirection :type ForwardBack%20Enum :default "ForwardBack_MAX") (TurnDirection :type LeftRIght%20Enum :default "NewEnumerator0"))
  (bind _returnvalue (Utilities|Select :Index TurnDirection :NewEnumerator0 -1.0 :NewEnumerator1 1.0))
  (bind _sphere (Variables|Default|GetSphere))
  (bind _turnpaddleforce (Variables|Default|GetTurnPaddleForce))
  (bind _returnvalue_2 (* _returnvalue _turnpaddleforce))
  (bind _out (Utilities|SaneTorque _returnvalue_2))
  ;[0 0.6818 1] Rowing Event - This is inefficient, get over it
  (Physics|AddForce _sphere (* (Math|Vector|GetForwardVector _sphere) (* (Utilities|SaneTorque (Variables|Default|GetMovementPaddleForce)) (Utilities|Select :Index PropulsionDirection :NewEnumerator0 1.0 :NewEnumerator1 -1.0))) "None" false)
  (Class|PrimitiveComponent|AddTorqueinRadians _sphere (Math|Vector|MakeVector 0.0 0.0 (Utilities|Select :Index PropulsionDirection :NewEnumerator0 _out :NewEnumerator1 (* _out -1.0))) "None" false))

(event Custom|UpgradeBoat
  (Utilities|GateServerOnly
    (:Authority
      (Transformation|AddRelativeLocation (Variables|Default|GetFront) "10.000000,10.000000,0.000000" false false)
      (Transformation|AddRelativeLocation (Variables|Default|GetTail) "0.000000,-20.000000, 0" false false)
      (bind _returnvalue (AddComponent|AddChildActorComponent false))
      (ChildActorComponent|SetChildActorClass _returnvalue "/Game/ThirdPersonCPP/Blueprints/BoatActorMethod/BP_Seat.BP_Seat_C")
      (Transformation|AttachComponentToComponent _returnvalue (Variables|Default|GetFront) "None" "KeepWorld" "KeepWorld" "KeepWorld" true)
      (Transformation|SetRelativeLocation _returnvalue (Variables|/Script/Engine.SceneComponent|GetRelativeLocation (Variables|Default|GetTail)) false false))))

(event EventTick
  (params (DeltaSeconds :type Float%20%28single-precision%29))
  (bind _sphere (Variables|Default|GetSphere))
  ;[1 1 1] LockWorldRotation
  (Transformation|SetWorldRotation _sphere (Math|Rotator|MakeRotator 0.0 0.0 (.yaw (Transformation|GetWorldRotation _sphere))) false false)
  (|AligntVelocityToBoatDirection DeltaSeconds))

(fn ConstructionScript)