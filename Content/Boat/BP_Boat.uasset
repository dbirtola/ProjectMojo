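; Multiplayer rowing boat that rams other boats and absorbs the crew of any it sinks.
; Paddle strokes push and turn a physics Sphere, while server Tick keeps it upright and steers velocity along the hull axis.
; Hull hits deal damage; a destroyed boat upgrades its attacker once per rower, adding a seat, length, mass and health.
; Transferred rowers are seated through pawn and seat queues that poll with delays until seats are valid.
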(event OnComponentHit(HitBox)
  (params (HitComponent :type Primitive%20Component%20Object%20Reference) (OtherActor :type Actor%20Object%20Reference) (OtherComp :type Primitive%20Component%20Object%20Reference) (NormalImpulse :type Vector :default "0, 0, 0") (Hit :type Hit%20Result%20Structure%20%28by%20ref%29))
  (Utilities|GateServerOnly
    (:Authority
      (bind _asbp_boat (Utilities|Casting|CastToBP_Boat OtherActor))
      (Game|Damage|ApplyDamage _asbp_boat 5e+01 0 self))))

(event Custom|MULTICAST_PlaceOar
  (params (ActorComp :type Child%20Actor%20Component%20Object%20Reference) (Attachee :type Actor%20Object%20Reference))
  (Default|AttachtoSeat (Utilities|NewMacro0 ActorComp) Attachee))

(event Custom|AttachToBoat
  (params (Attachee :type Actor%20Object%20Reference))
  (bind _queue (Variables|Default|GetQueue))
  (bind _childactorqueue (Variables|Default|GetChildActorQueue))
  (bind _output (Utilities|Array|Get(acopy) _childactorqueue))
  (bind _asbp_seat (Utilities|NewMacro0 _output))
  (bind _asbp_boater_pawn (Utilities|Casting|CastToBP_BoaterPawn Attachee))
  (Utilities|Array|Add _queue _asbp_boater_pawn)
  (if (Variables|Default|GetWorking) :!label _label
    (Utilities|FlowControl|Delay 0.2)
    (if (> (Utilities|Array|Length _queue) 0)
      (goto _label))
    (else
      (Variables|Default|SetWorking true)
      (Utilities|IsValid _asbp_seat :!label _label_2
        (:Is%20Valid
          (Default|AttachtoSeat _asbp_seat (Utilities|Array|Get(acopy) (Variables|Default|GetQueue)))
          (Utilities|Array|Add (Variables|Default|GetAttachedPlayers) (Utilities|Array|Get(acopy) (Variables|Default|GetQueue)))
          (Variables|/Game/Player/BP_BoaterPawn.BP_BoaterPawn_C|SetBoat (Utilities|Array|Get(acopy) (Variables|Default|GetQueue)) self)
          (Utilities|Array|RemoveIndex (Variables|Default|GetQueue))
          (Utilities|Array|RemoveIndex (Variables|Default|GetChildActorQueue))
          (Variables|Default|SetWorking false))
        (:Is%20Not%20Valid
          (Utilities|FlowControl|Delay 0.2)
          (goto _label_2))))))

(event Custom|UpgradeBoat
  (bind _hitbox (Variables|Default|GetHitBox))
  (bind _relativescale3d (Variables|/Script/Engine.SceneComponent|GetRelativeScale3D _hitbox))
  (Utilities|GateServerOnly
    (:Authority
      (Transformation|AddRelativeLocation (Variables|Default|GetFront) "10.000000,0.000000,0.000000" false false)
      (Transformation|AddRelativeLocation (Variables|Default|GetTail) "0.000000,-20.000000, 0" false false)
      (bind _returnvalue (AddComponent|AddChildActorComponent false))
      (Utilities|Array|Add (Variables|Default|GetChildActorQueue) _returnvalue)
      (ChildActorComponent|SetChildActorClass _returnvalue "/Game/ThirdPersonCPP/Blueprints/BoatActorMethod/BP_Seat.BP_Seat_C")
      (Transformation|AttachComponentToComponent _returnvalue (Variables|Default|GetFront) "None" "KeepWorld" "KeepWorld" "KeepWorld" true)
      (Transformation|SetRelativeTransform _returnvalue (Math|Transform|MakeTransform (Variables|/Script/Engine.SceneComponent|GetRelativeLocation (Variables|Default|GetTail)) "0, 0, 0" "1,1,1") false false)
      (Transformation|SetRelativeScale3D _hitbox (Math|Vector|MakeVector (.x _relativescale3d) (.y _relativescale3d) (+ (.z _relativescale3d) 0.2)))
      (Class|PrimitiveComponent|SetMassOverrideinKg _hitbox "None" (+ (Physics|GetMass _hitbox) 5e+01) true)
      (bind _output_get (Variables|Default|SetMaxBoatHealth (+ (Variables|Default|GetMaxBoatHealth) (Variables|Default|GetUpgradeHealthIncreaseValue))))
      (Variables|Default|SetBoatHealth _output_get)
      (Utilities|FlowControl|Delay 0.2))))

(event Custom|Row!
  (params (PropulsionDirection :type ForwardBack%20Enum :default "ForwardBack_MAX") (TurnDirection :type LeftRIght%20Enum :default "NewEnumerator0"))
  (bind _returnvalue (Utilities|Select :Index TurnDirection :NewEnumerator0 -1.0 :NewEnumerator1 1.0))
  (bind _sphere (Variables|Default|GetSphere))
  (bind _turnpaddleforce (Variables|Default|GetTurnPaddleForce))
  (bind _returnvalue_2 (* _returnvalue _turnpaddleforce))
  (bind _out (Utilities|SaneTorque _returnvalue_2))
  ;[0 0.6818 1] Rowing Event - This is inefficient, get over it
  (Physics|AddForce _sphere (* (Math|Vector|GetForwardVector _sphere) (* (Utilities|SaneTorque (Variables|Default|GetMovementPaddleForce)) (Utilities|Select :Index PropulsionDirection :NewEnumerator0 1.0 :NewEnumerator1 -1.0))) "None" false)
  (Class|PrimitiveComponent|AddTorqueinRadians _sphere (Math|Vector|MakeVector 0.0 0.0 (Utilities|Select :Index PropulsionDirection :NewEnumerator0 _out :NewEnumerator1 (* _out -1.0))) "None" false))

(event Custom|AttachToBoatInitial
  (params (Attachee :type Actor%20Object%20Reference))
  (bind _mid1 (Variables|Default|GetMid1))
  (bind _asbp_seat (Utilities|NewMacro0 _mid1))
  (Utilities|IsValid _asbp_seat :!label _label
    (:Is%20Valid
      (Default|AttachtoSeat _asbp_seat Attachee)
      (bind _asbp_boater_pawn (Utilities|Casting|CastToBP_BoaterPawn Attachee))
      (Utilities|Array|Add (Variables|Default|GetAttachedPlayers) _asbp_boater_pawn)
      (Variables|/Game/Player/BP_BoaterPawn.BP_BoaterPawn_C|SetBoat _asbp_boater_pawn self))
    (:Is%20Not%20Valid
      (Utilities|FlowControl|Delay 0.2)
      (goto _label))))

(event EventTick
  (params (DeltaSeconds :type Float%20%28single-precision%29))
  (bind _sphere (Variables|Default|GetSphere))
  ;[1 1 1] LockWorldRotation
  (Utilities|GateServerOnly
    (:Authority
      (Transformation|SetWorldRotation _sphere (Math|Rotator|MakeRotator 0.0 0.0 (.yaw (Transformation|GetWorldRotation _sphere))) false false)
      (|AligntVelocityToBoatDirection DeltaSeconds))))

(event Game|Damage|EventAnyDamage
  (params (Damage :type Float%20%28single-precision%29) (DamageType :type Damage%20Type%20Object%20Reference) (InstigatedBy :type Controller%20Object%20Reference) (DamageCauser :type Actor%20Object%20Reference))
  (Utilities|GateServerOnly
    (:Authority
      (bind _asbp_boat (Utilities|Casting|CastToBP_Boat DamageCauser))
      (bind _output_get (Variables|Default|SetBoatHealth (- (Variables|Default|GetBoatHealth) (Math|Float|Truncate Damage))))
      (if (<= _output_get 0)
        (for _array_element (Variables|Default|GetAttachedPlayers)
          (CallFunction|UpgradeBoat _asbp_boat)
          (CallFunction|AttachtoBoat _asbp_boat _array_element))
        (CallFunction|KillBoat)))))

(fn ConstructionScript)

(fn DealDamage
  (params (Damage :type Integer))
  (bind _output_get (Variables|Default|SetBoatHealth (- (Variables|Default|GetBoatHealth) Damage)))
  (if (<= _output_get 0)
    (CallFunction|KillBoat)))

(fn KillBoat
  (Actor|DestroyActor))