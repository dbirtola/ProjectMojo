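; Player pawn for a boater that rows a BP_Boat, forwarding left and right strokes with a reverse option and playing the oar animations.
; On BeginPlay a dedicated server spawns the boat at the pawn's transform, while other instances poll until the Boat reference is valid; both then attach to it.
; Boat upgrades are forwarded to the boat only on the server.
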(event Custom|RightRow
  (params (Reverse? :type Boolean))
  (Default|Row! (Variables|Default|GetBoat) (select Reverse? "NewEnumerator1" "NewEnumerator0") "NewEnumerator1")
  (Default|RowAnimationForwardRight (Utilities|GetOar)))

(event Custom|LeftRow
  (params (Reverse? :type Boolean))
  (Default|Row! (Variables|Default|GetBoat) (select Reverse? "NewEnumerator1" "NewEnumerator0") "NewEnumerator0")
  (Default|RowAnimationForwardLeft (Utilities|GetOar)))

(event Custom|UpgradeBoat
  (Utilities|GateServerOnly
    (:Authority
      (Default|UpgradeBoat (Variables|Default|GetBoat)))))

(event EventBeginPlay
  ;[1 1 1] We server?
  (if (Networking|IsDedicatedServer)
    (bind _returnvalue (Game|SpawnActorfromClass "/Game/Boat/BP_Boat.BP_Boat_C" (Transformation|GetActorTransform self) "Undefined" 0 0))
    (bind _output_get (Variables|Default|SetBoat _returnvalue))
    (else
      (Utilities|IsValid (Variables|Default|GetBoat) :!label _label
        (:Is%20Valid
          _)
        (:Is%20Not%20Valid
          (Utilities|FlowControl|Delay 0.2)
          (goto _label)))))
  (Default|AttachtoBoatInitial _output_get self))

(fn ConstructionScript)