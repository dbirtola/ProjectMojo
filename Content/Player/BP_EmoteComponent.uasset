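; BP_EmoteComponent is a component intended to show player emotes as screen widgets.
; BroadcastEmoteToPlayers loops over the PlayerArray on the authority and casts each pawn to BP_BoaterPawn, but takes no further action.
; On non-authority instances, ReceiveEmote creates the given widget class for the owning pawn's controller.
; It offsets the widget once to the emoting pawn's projected location and adds it to that player's screen.
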(event Custom|BroadcastEmoteToPlayers
  (params (InputWidget :type User%20Widget%20Class%20Reference) (EmotingPawn :type BP%20Boater%20Pawn%20Object%20Reference))
  (if (Ability|HasAuthority (Components|GetOwner))
    (for _array_element (Variables|/Script/Engine.GameStateBase|GetPlayerArray (Game|GetGameState))
      (Utilities|Casting|CastToBP_BoaterPawn (Variables|/Script/Engine.PlayerState|GetPawnPrivate _array_element)))))

(event Custom|ReceiveEmote
  (params (InputWidgetClass :type User%20Widget%20Class%20Reference) (EmotingPawn :type BP%20Boater%20Pawn%20Object%20Reference))
  (bind _returnvalue (Components|GetOwner))
  (if (not (Ability|HasAuthority _returnvalue))
    (bind _aspawn (Utilities|Casting|CastToPawn _returnvalue))
    (bind _asplayer_controller (Utilities|Casting|CastToPlayerController (Pawn|GetController _aspawn)))
    (bind _returnvalue_2 (UserInterface|CreateWidget InputWidgetClass _asplayer_controller))
    (Class|Widget|SetRenderTranslation _returnvalue_2 (.ScreenPosition (Class|GameplayStatics|ProjectWorldtoScreen _asplayer_controller (Transformation|GetActorLocation EmotingPawn) false)))
    (UserInterface|Viewport|AddtoPlayerScreen _returnvalue_2)))

(event EventBeginPlay)

(event EventTick
  (params (DeltaSeconds :type Float%20%28single-precision%29)))