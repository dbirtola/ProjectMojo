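; Player controller for the rowing boat that turns left and right paddle input into Row calls on the possessed BP_BoaterPawn.
; Possession creates two paused looping timers, one per side, which paddle presses unpause and releases pause to repeat strokes, with a reverse modifier.
; Paddle input acts only on remote clients.
; When forward input is required but not held, paddle presses set that side's brake flag instead.
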(event Custom|RightRow
  (params (Reverse? :type Boolean))
  (bind _boater (Variables|Default|GetBoater))
  (Utilities|IsValid _boater
    (:Is%20Valid
      (Default|Row! (Variables|/Game/Player/BP_BoaterPawn.BP_BoaterPawn_C|GetTempFollow _boater) (select Reverse? "NewEnumerator1" "NewEnumerator0") "NewEnumerator1"))))

(event Custom|LeftRow
  (params (Reverse? :type Boolean))
  (bind _boater (Variables|Default|GetBoater))
  (Utilities|IsValid _boater
    (:Is%20Valid
      (Default|Row! (Variables|/Game/Player/BP_BoaterPawn.BP_BoaterPawn_C|GetTempFollow _boater) (select Reverse? "NewEnumerator1" "NewEnumerator0") "NewEnumerator0"))))

(event Custom|PossessPawn
  (params (Pawn :type Pawn%20Object%20Reference))
  (bind _returnvalue (Pawn|GetControlledPawn))
  (Utilities|FlowControl|Sequence
    (:then_0
      (Utilities|IsValid _returnvalue
        (:Is%20Valid
          (Actor|DestroyActor _returnvalue))))
    (:then_1
      (Pawn|Possess Pawn))))

(event Custom|ClientLeftRow
  (CallFunction|LeftRow (Variables|Input|GetReverse?)))

(event Custom|ClientRightRow
  (CallFunction|RightRow (Variables|Input|GetReverse?)))

(event EventPossess
  (params (PossessedPawn :type Pawn%20Object%20Reference))
  (bind _asbp_boater_pawn (Utilities|Casting|CastToBP_BoaterPawn PossessedPawn))
  (Variables|Default|SetBoater _asbp_boater_pawn)
  (bind _returnvalue (Utilities|Time|SetTimerbyEvent (delegate Custom|ClientLeftRow) 0.3 true 0.5))
  (bind _output_get (Variables|Timer|SetLeftRowTimer _returnvalue))
  (Utilities|Time|PauseTimerbyHandle _output_get)
  (bind _returnvalue_2 (Utilities|Time|SetTimerbyEvent (delegate Custom|ClientRightRow) 0.3 true 0.5))
  (bind _output_get_2 (Variables|Timer|SetRightRowTimer _returnvalue_2))
  (Utilities|Time|PauseTimerbyHandle _output_get_2))

(event Input|ActionEvents|InputActionPaddleLeft
  (params (Key :type Key%20Structure :default "None"))
  (:Pressed
    ;[0 1 0.03953] Ensure input is coming from client
    (Networking|SwitchHasAuthority
      (:Remote
        (if (Variables|Brake|GetForwardInputRequiredToRow)
          (if (Variables|Input|GetbForwardInput)
            (Utilities|Time|UnpauseTimerbyHandle (Variables|Timer|GetLeftRowTimer) :!label _label)
            (else
              (Variables|Brake|SetBrakeLeft true)
              (Variables|Brake|SetBrakeRight false)))
          (else
            (goto _label))))))
  (:Released
    (Utilities|Time|PauseTimerbyHandle (Variables|Timer|GetLeftRowTimer))
    (Variables|Brake|SetBrakeLeft false)))

(event Input|ActionEvents|InputActionPaddleRight
  (params (Key :type Key%20Structure :default "None"))
  (:Pressed
    ;[0 1 0.03953] Ensure input is coming from client
    (Networking|SwitchHasAuthority
      (:Remote
        (if (Variables|Brake|GetForwardInputRequiredToRow)
          (if (Variables|Input|GetbForwardInput)
            (Utilities|Time|UnpauseTimerbyHandle (Variables|Timer|GetRightRowTimer) :!label _label)
            (else
              (Variables|Brake|SetBrakeRight true)
              (Variables|Brake|SetBrakeLeft false)))
          (else
            (goto _label))))))
  (:Released
    (Utilities|Time|PauseTimerbyHandle (Variables|Timer|GetRightRowTimer))
    (Variables|Brake|SetBrakeRight false)))

(event Input|ActionEvents|InputActionReversePaddle
  (params (Key :type Key%20Structure :default "None"))
  (:Pressed
    ;[0 1 0.03953] Ensure input is coming from client
    (Networking|SwitchHasAuthority
      (:Remote
        (Variables|Input|SetReverse? true))))
  (:Released
    (Networking|SwitchHasAuthority
      (:Remote
        (Variables|Input|SetReverse? false)))))

(event Input|ActionEvents|InputActionUpArrow
  (params (Key :type Key%20Structure :default "None"))
  (:Pressed
    (Variables|Input|SetbForwardInput true))
  (:Released
    (Variables|Input|SetbForwardInput false)))

(fn ConstructionScript)